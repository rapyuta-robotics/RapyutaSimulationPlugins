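; ROS 2-controlled AI character that walks to goals using AIMoveTo, with idle and walk animations.
; On BeginPlay it resolves origin-relative goals, reads JSON spawn parameters from ROS2Spawnable, and registers ROS 2 subscribers for goals, mode and speed, plus a move-status publisher.
; While idle, Tick waits an interval, then picks the next move by mode: sequential goal, random goal, or random bounding-box point; mode 0 has no automatic move.
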(event `self.ReceiveBeginPlay`
  (bind _originbyactor (`self.OriginByActor`))
  (bind _publisher (`ROS2PublisherComponent.Publisher` (`self.MoveStatusPublisher`)))
  (bind _subscriber (`ROS2SubscriberComponent.Subscriber` (`self.ActorNameGoalSubscriber`)))
  (bind _subscriber_2 (`ROS2SubscriberComponent.Subscriber` (`self.SetModeSubscriber`)))
  (bind _subscriber_3 (`ROS2SubscriberComponent.Subscriber` (`self.SetVelSubscriber`)))
  (bind _subscriber_4 (`ROS2SubscriberComponent.Subscriber` (`self.PoseGoalSubscriber`)))
  (`|ExecutionSequence`
    (:`then_0`
      ;[1 1 1] Convert Actor to location and world location to relative location
      (`/Engine/EditorBlueprintResources/StandardMacros.IsValid` _originbyactor
        (:`Is Valid`
          (set `self.Origin` (`self.GetTransform` _originbyactor)))))
    (:`then_1`
      (`self.TransfromGoalSequenceToWorldCoordinate`)
      (for _array_element (`self.GoalSequenceName`)
        (`/Engine/EditorBlueprintResources/StandardMacros.IsValid` _array_element
          (:`Is Valid`
            (`KismetArrayLibrary.Array_Add` (`self.GoalSequence`) (`self.K2_GetActorLocation` _array_element))))))
    (:`then_2`
      (`self.ROSParamParser`))
    (:`then_3`
      (set `self.CurrentGoal` (`self.K2_GetActorLocation`))
      (if (`self.UIWidgetEnabled`)
        (`RRUIWidgetComponent.Init` (`self.RRUIWidget`))
        (`self.SpawnDefaultController`)
        (`KismetSystemLibrary.PrintString` (`KismetStringLibrary.Conv_IntToString` (`self.Mode`)))))
    (:`then_4`
      (`self.OnMoveCompoleted`))
    (:`then_5`
      (`|ExecutionSequence`
        (:`then_1`
          (`ROS2NodeComponent.Init` (`self.ROS2Node`)))
        (:`then_2`
          (`|ExecutionSequence`
            (:`then_0`
              (`ROS2Subscriber.SetDelegates` _subscriber_4 (delegate `PoseGoalCallback`))
              (`ROS2NodeComponent.AddSubscription` (`self.ROS2Node`) _subscriber_4))
            (:`then_1`
              (`ROS2Subscriber.SetDelegates` _subscriber (delegate `ActorNameGoalCallback`))
              (`ROS2NodeComponent.AddSubscription` (`self.ROS2Node`) _subscriber))))
        (:`then_3`
          (`ROS2Publisher.SetDelegates` _publisher (delegate `movestatusupdate`))
          (`ROS2NodeComponent.AddPublisher` (`self.ROS2Node`) _publisher))
        (:`then_4`
          (`|ExecutionSequence`
            (:`then_0`
              (`ROS2Subscriber.SetDelegates` _subscriber_2 (delegate `CustomEvent_1`))
              (`ROS2NodeComponent.AddSubscription` (`self.ROS2Node`) _subscriber_2))
            (:`then_1`
              (`ROS2Subscriber.SetDelegates` _subscriber_3 (delegate `CustomEvent_0`))
              (`ROS2NodeComponent.AddSubscription` (`self.ROS2Node`) _subscriber_3))))))))

(event `PoseGoalCallback`
  (params (InMessage :type "ROS2GenericMsg Object Reference"))
  (bind _output (`ROS2PoseStampedMsg.GetMsg` (cast `ROS2PoseStampedMsg` InMessage :!pure true)))
  (bind _returnvalue (`RRConversionUtils.VectorROSToUE` (break `ROSPose` (`.Pose` (break `ROSPoseStamped` _output)))))
  (bind _returnvalue_2 (`RRGeneralUtils.GetWorldTransformFromName` (`.FrameId` (break `ROSHeader` (break `ROSPoseStamped` _output))) (`KismetMathLibrary.MakeTransform` _returnvalue)))
  (`self.MoveTo` (.location _returnvalue_2)))

(event `ActorNameGoalCallback`
  (params (InMessage :type "ROS2GenericMsg Object Reference"))
  (bind _output_data (break `ROSStr` (`ROS2StrMsg.GetMsg` (cast `ROS2StrMsg` InMessage :!pure true))))
  (bind _returnvalue (`RRGeneralUtils.FindActorByName` _output_data "CaseSensitive"))
  (`/Engine/EditorBlueprintResources/StandardMacros.IsValid` _returnvalue
    (:`Is Valid`
      (`self.MoveTo` (0.0 0.0 0.0) _returnvalue))))

(event `movestatusupdate`
  (params (InTopicMessage :type "ROS2GenericMsg Object Reference"))
  (`ROS2Int32Msg.SetMsg` (cast `ROS2Int32Msg` InTopicMessage :!pure true) (make `ROSInt32` (`self.MoveStatus`))))

(event `CustomEvent_1`
  (params (InMessage :type "ROS2GenericMsg Object Reference"))
  (bind _output_data (break `ROSInt32` (`ROS2Int32Msg.GetMsg` (cast `ROS2Int32Msg` InMessage :!pure true))))
  (`self.ModeTransition` _output_data))

(event `CustomEvent_0`
  (params (InMessage :type "ROS2GenericMsg Object Reference"))
  (bind _output_data (break `ROSFloat32` (`ROS2Float32Msg.GetMsg` (cast `ROS2Float32Msg` InMessage :!pure true))))
  (`self.SetSpeed` _output_data))

(event `self.ReceiveTick`
  (params (DeltaSeconds :type "Float (single-precision)"))
  ;[1 1 1] Check whether character reach goal
  (if (== (`self.MoveStatus`) 0)
    (if (>= (`GameplayStatics.GetTimeSeconds`) (+ (`self.LastMoveCompletedTime`) (`self.AutoMoveInterval`)))
      ;[1 1 1] Change behaviour based on mode
      (`self.ShiftToNextMove`))))

(fn `Add Sequence By Actor`
  (params (TargetActor :type "Actor Object Reference"))
  (`/Engine/EditorBlueprintResources/StandardMacros.IsValid` TargetActor
    (:`Is Valid`
      (`KismetArrayLibrary.Array_Add` (`self.GoalSequence`) (`self.K2_GetActorLocation` TargetActor)))
    (:`Is Not Valid`
      (`/RapyutaSimulationPlugins/Tools/RRGeneralUtility.DebugNamed Log` "Given Actor is not valid" self))))

(fn `Add Sequence By Name`
  (params (TargetActorName :type String))
  (bind _returnvalue (`RRGeneralUtils.FindActorByName` TargetActorName))
  (`self.Add Sequence By Actor` _returnvalue))

(fn `Add SequenceFromRelativePose`
  (params (RelativePose :type "Vector Structure"))
  (bind _returnvalue (`RRGeneralUtils.GetWorldTransform` (`self.Origin`) (`KismetMathLibrary.MakeTransform` RelativePose)))
  (`KismetArrayLibrary.Array_Add` (`self.GoalSequence`) (.location _returnvalue)))

(fn `ModeTransition`
  (params (InputPin :type Integer))
  (if (> InputPin 3)
    (`/RapyutaSimulationPlugins/Tools/RRGeneralUtility.Named Log` "Mode must be 0, 1" self :!label _label)
    (elif (< InputPin 0)
      (goto _label)
      (elif (not (== InputPin (`self.Mode`)))
        (bind _output_get (set `self.Mode` InputPin))
        (`/RapyutaSimulationPlugins/Tools/RRGeneralUtility.Named Log` (`KismetStringLibrary.Concat_StrStr` "mode was changed to" (`KismetStringLibrary.Conv_IntToString` _output_get)) self)
        ;[1 1 1] Initialize if mode change to 1,2,3
        (if (> InputPin 0)
          (set `self.GoalIndex` 0)
          (`self.OnMoveCompoleted`))))))

(fn `SetSpeed`
  (params (A :type "Float (double-precision)"))
  (bind _returnvalue (* A 100.0))
  (set `CharacterMovementComponent.MaxWalkSpeed` _returnvalue (`self.CharacterMovement`))
  (`/RapyutaSimulationPlugins/Tools/RRGeneralUtility.Named Log` (`KismetStringLibrary.Concat_StrStr` "speed was changed to " (`KismetStringLibrary.Conv_DoubleToString` _returnvalue)) self))

(fn `TransfromGoalSequenceToWorldCoordinate`
  (bind _tempgoal_sequence (`self.TempGoal Sequence`))
  (`KismetArrayLibrary.Array_Clear` _tempgoal_sequence)
  (`KismetArrayLibrary.Array_Resize` _tempgoal_sequence (`KismetArrayLibrary.Array_Length` (`self.GoalSequence`)))
  (for (_array_element _array_index) (`self.GoalSequence`)
    (bind _returnvalue (`RRGeneralUtils.GetWorldTransform` (`self.Origin`) (`KismetMathLibrary.MakeTransform` _array_element)))
    (`KismetArrayLibrary.Array_Set` (`self.TempGoal Sequence`) _array_index (.location _returnvalue)))
  (set `self.GoalSequence` (`self.TempGoal Sequence`)))

(fn `UpdateGoalIndex`
  (returns (Output_Get :type Integer))
  (bind _returnvalue (+ (`self.GoalIndex`) 1))
  (if (> _returnvalue (- (`KismetArrayLibrary.Array_Length` (`self.GoalSequence`)) 1))
    (bind _output_get (set `self.GoalIndex` 0))
    (return _output_get)
    (else
      (bind _output_get_2 (set `self.GoalIndex` _returnvalue))
      (return _output_get_2))))

(fn `UserConstructionScript`)