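; Simple ROS-controlled AI character that navigates by mode, origin and goal sequence, and can pick and drop payloads.
; BeginPlay spawns its controller and, unless ROS-spawned, pushes placed movement settings to it, resolving relative goals to world transforms.
; ROSParamParser reads ROS2Spawnable JSON, converting ROS coordinates or resolving actor names.
; Pick/drop events forward to BP_RRROS2AIController, using Cylinder as attachment link; animation updating is unwired.
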(event `self.ReceiveBeginPlay`
  (bind _returnvalue (`self.GetComponentByClass` "/Script/RapyutaSimulationPlugins.ROS2Spawnable"))
  (bind _originbyactor (`self.OriginByActor`))
  (bind _rosaicontroller (`self.ROSAIController`))
  (bind _rosaicontroller_2 (`self.ROSAIController`))
  (bind _rosaicontroller_3 (`self.ROSAIController`))
  (`|ExecutionSequence`
    (:`then_0`
      (`self.SpawnDefaultController`)
      (bind _asrrairobot_roscontroller (cast `RRAIRobotROSController` (`self.GetController`)))
      (set `self.ROSAIController` _asrrairobot_roscontroller))
    (:`then_1`
      (`/Engine/EditorBlueprintResources/StandardMacros.IsValid` _returnvalue
        (:`Is Valid`
          (bind _outjsonobject (`JsonBlueprintFunctionLibrary.FromString` (`ROS2Spawnable.ActorJsonConfigs` _returnvalue)))
          (bind (_outvalue _returnvalue_2) (`|GetJsonField` _outjsonobject "enable_widget"))
          (if _returnvalue_2
            (set `self.UIWidgetEnabled` _outvalue)))
        (:`Is Not Valid`
          (`/Engine/EditorBlueprintResources/StandardMacros.IsValid` (`self.ROSAIController`)
            (:`Is Valid`
              (`|ExecutionSequence`
                (:`then_0`
                  ;[1 1 1] Convert Actor to location and world location to relative location, and set param to controller
                  (`/Engine/EditorBlueprintResources/StandardMacros.IsValid` _originbyactor
                    (:`Is Valid`
                      (set `RRAIRobotROSController.OriginActor` _originbyactor _rosaicontroller_3))
                    (:`Is Not Valid`
                      (set `RRAIRobotROSController.Origin` (`self.Origin`) _rosaicontroller_3))))
                (:`then_1`
                  (`KismetArrayLibrary.Array_Clear` (`RRAIRobotROSController.GoalSequence` (`self.ROSAIController`)))
                  (for _array_element (`self.GoalSequence`)
                    (bind _returnvalue_3 (`RRAIRobotROSController.GetOrigin` _rosaicontroller))
                    (bind _returnvalue_4 (`RRGeneralUtils.GetWorldTransform` _returnvalue_3 _array_element))
                    (`KismetArrayLibrary.Array_Add` (`RRAIRobotROSController.GoalSequence` _rosaicontroller) _returnvalue_4))
                  (for _array_element_2 (`self.GoalSequenceName`)
                    (`/Engine/EditorBlueprintResources/StandardMacros.IsValid` _array_element_2
                      (:`Is Valid`
                        (`KismetArrayLibrary.Array_Add` (`RRAIRobotROSController.GoalSequence` (`self.ROSAIController`)) (`self.GetTransform` _array_element_2))))))
                (:`then_2`
                  (set `RRAIRobotROSController.RandomMoveBoundingBox` (`self.RandomMoveBoundingBoxSize`) _rosaicontroller_2)
                  (set `RRAIRobotROSController.Mode` (`self.Mode`) _rosaicontroller_2))))))))
    (:`then_2`
      (if (`self.UIWidgetEnabled`)
        (`RRUIWidgetComponent.Init` (`self.RRUIWidget`))))))

(event `self.ReceiveTick`
  (params (DeltaSeconds :type "Float (single-precision)")))

(event `self.ReceivePossessed`
  (params (NewController :type "Controller Object Reference"))
  (bind _asbp_rrros2aicontroller (cast `/RapyutaSimulationPlugins/AI/BP_RRROS2AIController` NewController))
  (set `/RapyutaSimulationPlugins/AI/BP_RRROS2AIController.DefaultPickDropParam` (`self.DefaultPickDropParam`) _asbp_rrros2aicontroller))

(event `DropEvent`
  (params (DropLocation :type "Transform Structure") (DropLocationActor :type "Actor Object Reference") (UseApproach :type Boolean) (ApproachLocation :type "Vector Structure") (ApproachLocationActor :type "Actor Object Reference") (UseDefaultApproach :type Boolean))
  (bind _asbp_rrros2aicontroller (cast `/RapyutaSimulationPlugins/AI/BP_RRROS2AIController` (`self.GetController`)))
  (`/RapyutaSimulationPlugins/AI/BP_RRROS2AIController.DropBTEvent` _asbp_rrros2aicontroller DropLocation DropLocationActor UseApproach ApproachLocation ApproachLocationActor UseDefaultApproach))

(event `PickEvent`
  (params (PayloadLocation :type "Vector Structure") (TargetPayload :type "Actor Object Reference") (UseApproach :type Boolean) (ApproachLocation :type "Vector Structure") (ApproachLocationActor :type "Actor Object Reference") (UseDefaultApproach :type Boolean))
  (bind _asbp_rrros2aicontroller (cast `/RapyutaSimulationPlugins/AI/BP_RRROS2AIController` (`self.GetController`)))
  (`/RapyutaSimulationPlugins/AI/BP_RRROS2AIController.PickBTEvent` _asbp_rrros2aicontroller PayloadLocation TargetPayload UseApproach ApproachLocation ApproachLocationActor UseDefaultApproach))

(fn `UpdateAnimation`
  (params (MoveStatus :type "EPathFollowingStatus Enum" :default "Idle"))
  (bind _mesh (`self.Mesh`))
  (switch `EPathFollowingStatus` MoveStatus
    (:`Idle`
      (`SkeletalMeshComponent.PlayAnimation` _mesh "/Game/Mannequins/Animations/Manny/MM_Idle.MM_Idle" true :!label _label))
    (:`Waiting`
      (goto _label))
    (:`Paused`
      (goto _label))
    (:`Moving`
      (`SkeletalMeshComponent.PlayAnimation` _mesh "/Game/Mannequins/Animations/Manny/MM_Walk_Fwd.MM_Walk_Fwd" true))))

(fn `UserConstructionScript`
  (set `/RapyutaSimulationPlugins/AI/BP_PickDropParam.AttachmentLink` (`self.Cylinder`) (`self.DefaultPickDropParam`)))