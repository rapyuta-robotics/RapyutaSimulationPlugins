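; AI controller for a ROS2 character that animates its hands to pick up and drop payload actors.
; Tick moves both hand targets linearly at constant speed from weapon socket start positions to goals, and refreshes pawn-relative carrying positions.
; PickAnim and DropAnim aim hands using payload handles, poll until they arrive, attach to hand_l or detach, then return toward carrying pose.
; DirectHandControl is enabled during these sequences.
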(event `DropAnimEvent`
  (params (Target :type "Actor Object Reference"))
  (`self.DropAnim` Target))

(event `PickAnimEvent`
  (params (Target :type "Actor Object Reference"))
  (`self.PickAnim` Target))

(event `self.ReceiveBeginPlay`
  (`parent.ReceiveBeginPlay`)
  (`self.UpdateCarryingPosition` :!label _label)
  (`self.SetHandToCarryingWithoutMove`)
  (`self.SetHandBeginPose`))

(event `self.ReceivePossess`
  (params (PossessedPawn :type "Pawn Object Reference"))
  (goto _label))

(event `self.ReceiveTick`
  (params (DeltaSeconds :type "Float (single-precision)"))
  (`parent.ReceiveTick` DeltaSeconds)
  (`self.UpdateCarryingPosition`)
  (set `self.HandMoving` false)
  (bind _y (`self.LinearUpdateGoal` (`self.HandMoveStartTime`) (`KismetSystemLibrary.GetGameTimeInSeconds`) (`self.LeftHandPositionBegin`) (`self.LeftHandPositionFinalGoal`) (`self.HandSpeed`)))
  (set `self.LeftHandPositionTarget` _y)
  (bind _y_2 (`self.LinearUpdateGoal` (`self.HandMoveStartTime`) (`KismetSystemLibrary.GetGameTimeInSeconds`) (`self.RightHandPositionBegin`) (`self.RightHandPositionFinalGoal`) (`self.HandSpeed`)))
  (set `self.RightHandPositionTarget` _y_2))

(fn `LinearUpdateGoal`
  (params (x0 :type "Float (double-precision)") (x :type "Float (double-precision)") (y0 :type "Vector Structure") (ye :type "Vector Structure") (dydx :type "Float (double-precision)"))
  (returns (y :type "Vector Structure"))
  (locals (Temp :type "Vector Structure"))
  (bind _returnvalue (- ye y0))
  (bind _returnvalue_2 (- x x0))
  (if (<= (`KismetMathLibrary.VSize` _returnvalue) 5.0)
    (set `local.Temp` ye :!label _label)
    (elif (> _returnvalue_2 (`KismetMathLibrary.VSize` (/ _returnvalue dydx)))
      (goto _label)
      (else
        (set `local.Temp` (+ y0 (* (`KismetMathLibrary.Normal` _returnvalue) (* _returnvalue_2 dydx))))
        (set `self.HandMoving` true))))
  (return (`local.Temp`)))

(fn `MoveHandToCarryingPose`
  (`self.SetHandBeginPose`)
  (`self.SetHandToCarryingWithoutMove`)
  (set `self.DirectHandControl` true))

(fn `SetHandBeginPose`
  (bind _asbp_roscharacter (cast `/RapyutaSimulationPlugins/Character/BP_ROSCharacter` (`self.K2_GetPawn`)))
  (bind _mesh (`Character.Mesh` _asbp_roscharacter))
  (set `self.LeftHandPositionBegin` (`SceneComponent.GetSocketLocation` _mesh "weapon_l"))
  (set `self.RightHandPositionBegin` (`SceneComponent.GetSocketLocation` _mesh "weapon_r"))
  (set `self.HandMoveStartTime` (`KismetSystemLibrary.GetGameTimeInSeconds`))
  (set `self.HandMoving` true))

(fn `SetHandToCarryingWithoutMove`
  (set `self.LeftHandPositionFinalGoal` (`self.LeftHandCarryingPosiiton`))
  (set `self.RightHandPositionFinalGoal` (`self.RightHandCarryingPosition`)))

(fn `UpdateCarryingPosition`
  (bind _returnvalue (`self.GetTransform` (`self.K2_GetPawn`)))
  (bind _returnvalue_2 (`RRGeneralUtils.GetWorldTransform` _returnvalue (`KismetMathLibrary.MakeTransform` (`self.LeftHandCarryingPosiitonOffset`))))
  (set `self.LeftHandCarryingPosiiton` (.location _returnvalue_2))
  (bind _returnvalue_3 (`RRGeneralUtils.GetWorldTransform` _returnvalue (`KismetMathLibrary.MakeTransform` (`self.RightHandCarryingPositionOffset`))))
  (set `self.RightHandCarryingPosition` (.location _returnvalue_3)))

(fn `UserConstructionScript`
  (`parent.UserConstructionScript`))