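; BP_PickDropParam is an AI parameter holder for pick and drop behavior, covering target distance, implement behaviors, offsets, heights and attachment points.
; Its CopyParam function copies these settings field by field from another instance, after checking that the source is valid.
; It has no other logic, as the event graph holds only disabled placeholder events.
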(fn `CopyParam`
  (params (Orig :type "/Game/AI/BP_PickDropParam Object Reference"))
  (`/Engine/EditorBlueprintResources/StandardMacros.IsValid` Orig
    (:`Is Valid`
      (set `self.DisToTarget` (`/Game/AI/BP_PickDropParam.DisToTarget` Orig))
      (set `self.PickImplBehavior` (`/Game/AI/BP_PickDropParam.PickImplBehavior` Orig))
      (set `self.DropImplBehavior` (`/Game/AI/BP_PickDropParam.DropImplBehavior` Orig))
      (set `self.PickOffset` (`/Game/AI/BP_PickDropParam.PickOffset` Orig))
      (set `self.ConveyHeight` (`/Game/AI/BP_PickDropParam.ConveyHeight` Orig))
      (set `self.IdleHeight` (`/Game/AI/BP_PickDropParam.IdleHeight` Orig))
      (set `self.ReachingOffset` (`/Game/AI/BP_PickDropParam.ReachingOffset` Orig))
      (set `self.AttachmentJoint` (`/Game/AI/BP_PickDropParam.AttachmentJoint` Orig))
      (set `self.AttachmentLink` (`/Game/AI/BP_PickDropParam.AttachmentLink` Orig)))))