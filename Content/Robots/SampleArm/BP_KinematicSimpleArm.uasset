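; BP_KinematicSimpleArm is a sample robot arm Blueprint made of four links chained by three joints.
; Its construction script sets the parent and child link on each joint, linking Link1 through Link4 in series.
; It then registers each joint by name in the Joints map.
; The event graph holds only empty placeholder events, so this Blueprint adds no runtime logic of its own.
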(fn `UserConstructionScript`
  (bind _joint12 (`self.Joint12`))
  (bind _joint23 (`self.Joint23`))
  (bind _joint34 (`self.Joint34`))
  (bind _joints (`self.Joints`))
  (`|ExecutionSequence`
    (:`then_0`
      (set `JointComponent.ParentLink` (`self.Link1`) _joint12)
      (set `JointComponent.ChildLink` (`self.Link2`) _joint12))
    (:`then_1`
      (set `JointComponent.ParentLink` (`self.Link2`) _joint23)
      (set `JointComponent.ChildLink` (`self.Link3`) _joint23))
    (:`then_2`
      (set `JointComponent.ParentLink` (`self.Link3`) _joint34)
      (set `JointComponent.ChildLink` (`self.Link4`) _joint34))
    (:`then_3`
      (`BlueprintMapLibrary.Map_Add` _joints "joint12" (`self.Joint12`))
      (`BlueprintMapLibrary.Map_Add` _joints "joint23" (`self.Joint23`))
      (`BlueprintMapLibrary.Map_Add` _joints "joint34" (`self.Joint34`)))))