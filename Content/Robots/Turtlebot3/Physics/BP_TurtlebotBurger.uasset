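; Blueprint for a Turtlebot3 Burger robot pawn driven by a TurtlebotROSController.
; On possession it casts the new controller to that class and clears its IsStatic flag.
; The construction script only prints whether such a controller is already attached, as a debug check.
; BeginPlay and Tick are empty, and a debug print of left and right wheel twist is left unconnected.
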(event `self.ReceivePossessed`
  (params (NewController :type "Controller Object Reference"))
  (bind _asturtlebot_roscontroller (cast `TurtlebotROSController` NewController))
  (set `TurtlebotROSController.IsStatic` false _asturtlebot_roscontroller))

(event `self.ReceiveBeginPlay`)

(event `self.ReceiveTick`
  (params (DeltaSeconds :type "Float (single-precision)")))

(fn `UserConstructionScript`
  (cast `TurtlebotROSController` (`self.GetController`)
    (:`then`
      (`KismetSystemLibrary.PrintString` "OK ---------------------------------------------"))
    (:`CastFailed`
      (`KismetSystemLibrary.PrintString` "nonnnnn !!!!!!!!!!!!!!!!!!!!!!!!!!!!!!!!!!!!!!"))))