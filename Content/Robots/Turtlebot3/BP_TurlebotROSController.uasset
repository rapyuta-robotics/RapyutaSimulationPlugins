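; Controller for a Turtlebot3 robot that bridges the possessed RobotVehicle pawn to ROS 2.
; On possess it initialises its child-actor ROS2 node, starts any lidar sensors attached to the pawn, and sets up odometry and TF publishers plus a /cmd_vel subscription.
; Twist messages become Unreal-space linear and angular velocities on the pawn.
; The odometry publisher's update delegate converts movement-component data to ROS and refreshes the TF.
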(event `self.ReceivePossess`
  (params (PossessedPawn :type "Pawn Object Reference"))
  (bind _odompublisher (`self.OdomPublisher`))
  (bind _asros2node (cast `ROS2Node` (`ChildActorComponent.ChildActor` (`self.ROS2Node`)) :!pure true))
  (`|ExecutionSequence`
    (:`then_0`
      ;[1 1 1] ROS Node Init
      (`ROS2Node.Init` _asros2node))
    (:`then_1`
      ;[1 1 1] Lidar
      (`self.InitLidar` _asros2node))
    (:`then_2`
      ;[1 1 1] Odom
      (set `ROS2Publisher.UpdateDelegate` (`|CreateDelegate` :!event `Odom Pub Update`) _odompublisher)
      (`ROS2Node.AddPublisher` _asros2node _odompublisher)
      (`ROS2Publisher.Init` _odompublisher "KeepLast")
      (`ROS2TFPublisher.InitTFPublisher` (`self.OdomTFPublisher`) _asros2node))
    (:`then_3`
      ;[1 1 1] cmd_vel call back
      (`ROS2Node.AddSubscription` _asros2node "/cmd_vel" "/Script/rclUE.ROS2TwistMsg" (`|CreateDelegate` :!event `Cmd Vel Cb`)))))

(event `self.ReceiveBeginPlay`)

(fn `Cmd Vel Cb`
  (params (Message :type "ROS2GenericMsg Object Reference"))
  (bind (_output_linear _output_angular) (break `ROSTwist` (`ROS2TwistMsg.GetMsg` (cast `ROS2TwistMsg` Message :!pure true))))
  (bind _asrobot_vehicle (cast `RobotVehicle` (`self.K2_GetPawn`) :!pure true))
  (`|ExecutionSequence`
    (:`then_0`
      (bind _returnvalue (`ConversionUtils.VectorROSToUE` _output_linear))
      (`RobotVehicle.SetLinearVel` _asrobot_vehicle _returnvalue))
    (:`then_1`
      (bind _returnvalue_2 (`ConversionUtils.RotationROSToUE` _output_angular))
      (`RobotVehicle.SetAngularVel` _asrobot_vehicle _returnvalue_2))))

(fn `InitLidar`
  (params (ROS2Node :type "ROS2Node Object Reference"))
  (for _array_element (`self.GetAttachedActors` (`self.K2_GetPawn`) true)
    (bind _assensor_lidar (cast `SensorLidar` _array_element))
    (`SensorLidar.InitToNode` _assensor_lidar ROS2Node)
    (`SensorLidar.Run` _assensor_lidar))
  (return))

(fn `Odom Pub Update`
  (params (TopicMessage :type "ROS2GenericMsg Object Reference"))
  (bind _robotvehiclemovecomponent (`RobotVehicle.RobotVehicleMoveComponent` (cast `RobotVehicle` (`self.K2_GetPawn`) :!pure true)))
  (`|ExecutionSequence`
    (:`then_0`
      ;[1 1 1] OdomTopic
      (bind _returnvalue (`ConversionUtils.OdomUEToROS` (`RobotVehicleMovementComponent.OdomData` _robotvehiclemovecomponent)))
      (`ROS2OdometryMsg.SetMsg` (cast `ROS2OdometryMsg` TopicMessage :!pure true) _returnvalue))
    (:`then_1`
      ;[1 1 1] Odom TF update
      (bind _returnvalue_2 (`RobotVehicleMovementComponent.GetOdomTF` _robotvehiclemovecomponent))
      (set `ROS2TFPublisher.TF` _returnvalue_2 (`self.OdomTFPublisher`)))))

(fn `UserConstructionScript`)