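; BP_PayloadBase is a base payload actor that exposes pick and drop points and can toggle its collision.
; On BeginPlay it disables collision if it has an attach parent actor.
; SetCollisionEnabled switches mesh components on itself and all recursively attached actors between QueryAndPhysics and NoCollision.
; Point getters find child actors by tag and parent component name; GetDropPoint also looks up an approach location in the DropApproachPoint map.
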(event `self.ReceiveBeginPlay`
  (`/Engine/EditorBlueprintResources/StandardMacros.IsValid` (`self.GetAttachParentActor`)
    (:`Is Valid`
      (`self.SetCollisionEnabled` false))))

(fn `GetDropPoint`
  (params (Name :type String))
  (returns (FoundActor :type "Actor Object Reference") (ApproachLocation :type "Actor Object Reference"))
  (bind _foundactor (`/RapyutaSimulationPlugins/Tools/RRGeneralUtility.GetChildActor` self "DropPoint" Name))
  (return _foundactor (`BlueprintMapLibrary.Map_Find` (`self.DropApproachPoint`) _foundactor)))

(fn `GetPickApproachPoint`
  (params (Name :type String))
  (returns (FoundActor :type "Actor Object Reference"))
  (return (`/RapyutaSimulationPlugins/Tools/RRGeneralUtility.GetChildActor` self "PickApproachPoint" Name)))

(fn `SetCollisionEnabled`
  (params (Enable :type Boolean))
  (for _array_element (`self.K2_GetComponentsByClass` "/Script/Engine.MeshComponent")
    (if Enable
      (`PrimitiveComponent.SetCollisionEnabled` _array_element "QueryAndPhysics")
      (else
        (`PrimitiveComponent.SetCollisionEnabled` _array_element "NoCollision"))))
  (for _array_element_2 (`self.GetAttachedActors` true true)
    (for _array_element_3 (`self.K2_GetComponentsByClass` _array_element_2 "/Script/Engine.MeshComponent")
      (if Enable
        (`PrimitiveComponent.SetCollisionEnabled` _array_element_3 "QueryAndPhysics")
        (else
          (`PrimitiveComponent.SetCollisionEnabled` _array_element_3 "NoCollision"))))))

(fn `UserConstructionScript`)