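; In-world transform gizmo that follows TargetActor, scales with player distance, and translates, scales or rotates it by dragging tagged handles.
; Mouse press takes the selected handle from BP_WidgetPlayer, highlights it, disables pawn input and opens a Tick gate until release.
; Translation and scale project mouse delta onto the screen-space axis.
; Rotation traces the cursor against a spawned hidden plane and applies angle deltas; older per-axis rotation code remains unused.
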(event `self.ReceiveTick`
  (params (DeltaSeconds :type "Float (single-precision)"))
  (bind _starttransform_location (`KismetMathLibrary.BreakTransform` (`self.StartTransform`)))
  (bind _targetactor (`self.TargetActor`))
  (bind _targetactor_2 (`self.TargetActor`))
  (bind (_starttransform_location_2 _starttransform_rotation _starttransform_scale) (`KismetMathLibrary.BreakTransform` (`self.StartTransform`)))
  (bind _selectedcomponent (`self.SelectedComponent`))
  (bind _targetactor_3 (`self.TargetActor`))
  (bind _selectedcomponent_2 (`self.SelectedComponent`))
  (bind (_normalizedvectorinviewport _normalizedvectorinworld) (`self.Get Orientation in View Port` (`self.DefaultSceneRoot`) _selectedcomponent_2))
  (bind (_returnvalue_location _returnvalue_rotation) (`KismetMathLibrary.BreakTransform` (`self.GetTransform` (`self.TargetActor`))))
  (bind _returnvalue_location_2 (`KismetMathLibrary.BreakTransform` (`SceneComponent.GetRelativeTransform` _selectedcomponent_2)))
  (`SceneComponent.K2_SetWorldTransform` (`self.DefaultSceneRoot`) (`KismetMathLibrary.MakeTransform` _returnvalue_location _returnvalue_rotation (* (`KismetMathLibrary.MakeVector` 1.0 1.0 1.0) (* (`KismetMathLibrary.VSize` (- (`self.K2_GetActorLocation` (`GameplayStatics.GetPlayerPawn` 0)) (`SceneComponent.K2_GetComponentLocation` (`self.DefaultSceneRoot`)))) (`self.ScalingFactor`)))) false false)
  (`/Engine/EditorBlueprintResources/StandardMacros.Gate` true :!label _label
    (:`Exit`
      ;[1 1 1] Mouse diff
      (bind _returnvalue (`WidgetLayoutLibrary.GetMousePositionOnViewport`))
      (if (`ActorComponent.ComponentHasTag` _selectedcomponent "translation")
        ;[1 1 1] Translation
        (`|ExecutionSequence`
          (:`then_0`
            (bind _returnvalue_2 (`KismetMathLibrary.DotProduct2D` (- _returnvalue (`self.StartMousePosition`)) _normalizedvectorinviewport))
            (bind _returnvalue_3 (+ _starttransform_location (* (* _normalizedvectorinworld _returnvalue_2) (`self.TransSensitivity`))))
            (`SceneComponent.K2_SetWorldLocation` (`self.DefaultSceneRoot`) _returnvalue_3 false false))
          (:`then_1`
            (`/Engine/EditorBlueprintResources/StandardMacros.IsValid` _targetactor_2
              (:`Is Valid`
                (`SceneComponent.K2_SetWorldLocation` (`Actor.RootComponent` _targetactor_2) _returnvalue_3 false false)))))
        (elif (`ActorComponent.ComponentHasTag` _selectedcomponent "scale")
          ;[1 1 1] Scale
          (`/Engine/EditorBlueprintResources/StandardMacros.IsValid` _targetactor
            (:`Is Valid`
              (`SceneComponent.SetWorldScale3D` (`Actor.RootComponent` _targetactor) (+ _starttransform_scale (* (* (`KismetMathLibrary.Normal` _returnvalue_location_2 0.001) _returnvalue_2) (`self.ScaleSensitivity`))))))
          (elif (`ActorComponent.ComponentHasTag` _selectedcomponent "rotation")
            ;[1 1 1] Rotation
            (`self.PreRotation2`)
            (bind (_start _end) (`self.GetStartEndVectorsInMarkerCoordinate2`))
            (`|ExecutionSequence`
              (:`then_0`
                (bind _returnvalue_4 (`KismetMathLibrary.RotatorFromAxisAndAngle` (`KismetMathLibrary.GetUpVector` (`SceneComponent.RelativeRotation` (`self.SelectedComponent`))) (- (`KismetMathLibrary.DegAtan2` (.x _start) (.y _start)) (`KismetMathLibrary.DegAtan2` (.x _end) (.y _end)))))
                (`SceneComponent.K2_AddLocalRotation` (`self.DefaultSceneRoot`) _returnvalue_4 false false))
              (:`then_1`
                (`/Engine/EditorBlueprintResources/StandardMacros.IsValid` _targetactor_3
                  (:`Is Valid`
                    (`SceneComponent.K2_AddLocalRotation` (`Actor.RootComponent` _targetactor_3) _returnvalue_4 false false)))))))))))

(event `IMLeftMouseClicked`
  (`self.DragStart`)
  (goto _label :!via `Open`))

(event `IMLeftMousesReleased`
  (`self.Released`)
  (goto _label :!via `Close`))

(event `self.XCylinder.OnClicked`
  (params (TouchedComponent :type "PrimitiveComponent Object Reference") (ButtonPressed :type "Key Structure"))
  ;[1 1 1] legacy
  (set `self.XSelected` true)
  (set `self.SelectedComponent` (`self.XCone`)))

(event `self.YCylinder.OnClicked`
  (params (TouchedComponent :type "PrimitiveComponent Object Reference") (ButtonPressed :type "Key Structure"))
  ;[1 1 1] legacy
  (set `self.YSelected` true)
  (set `self.SelectedComponent` null))

(event `self.ZCylinder.OnClicked`
  (params (TouchedComponent :type "PrimitiveComponent Object Reference") (ButtonPressed :type "Key Structure"))
  ;[1 1 1] legacy
  (set `self.ZSelected` true)
  (set `self.SelectedComponent` null))

(fn `DragStart`
  (bind _returnvalue (`GameplayStatics.GetPlayerController` 0))
  (bind _targetactor (`self.TargetActor`))
  (`KismetSystemLibrary.PrintString` "IM: Drag start")
  (`|ExecutionSequence`
    (:`then_0`
      (`/Engine/EditorBlueprintResources/StandardMacros.IsValid` _targetactor
        (:`Is Valid`
          (set `self.StartTransform` (`SceneComponent.K2_GetComponentToWorld` (`Actor.RootComponent` _targetactor))))))
    (:`then_1`
      (bind _returnvalue_2 (`WidgetLayoutLibrary.GetMousePositionOnViewport`))
      (set `self.StartMousePosition` _returnvalue_2))
    (:`then_2`
      (bind _output_get (set `self.PlaeyrPawn` (`GameplayStatics.GetPlayerPawn` 0)))
      (`self.DisableInput` _output_get _returnvalue))
    (:`then_3`
      (bind _output_get_2 (set `self.SelectedComponent` (cast `StaticMeshComponent` (`/RapyutaSimulationPlugins/Tools/BP_WidgetPlayer.SelectedInteractiveMarkerComponent` (cast `/RapyutaSimulationPlugins/Tools/BP_WidgetPlayer` _returnvalue :!pure true)) :!pure true)))
      (`self.SetMaterials` _output_get_2 (`|MakeMap` "x" "/RapyutaSimulationPlugins/Tools/MI_MarkerRedClicked.MI_MarkerRedClicked" "y" "/RapyutaSimulationPlugins/Tools/MI_MarkerGreenClicked.MI_MarkerGreenClicked" "z" "/RapyutaSimulationPlugins/Tools/MI_MarkerBlueClicked.MI_MarkerBlueClicked" :!type "Name" :!valuetype "MaterialInterface Object Reference")))))

(fn `Get Orientation in View Port`
  (params (Start :type "SceneComponent Object Reference (by ref)") (End :type "StaticMeshComponent Object Reference (by ref)"))
  (returns (NormalizedVectorInViewport :type "Vector2D Structure") (NormalizedVectorInWorld :type "Vector Structure"))
  (bind _returnvalue (`GameplayStatics.GetPlayerController` 0))
  (bind _returnvalue_2 (`SceneComponent.K2_GetComponentLocation` Start))
  (bind _returnvalue_3 (`SceneComponent.K2_GetComponentLocation` End))
  (return (`KismetMathLibrary.Normal2D` (- (`WidgetLayoutLibrary.ProjectWorldLocationToWidgetPosition` _returnvalue _returnvalue_3) (`WidgetLayoutLibrary.ProjectWorldLocationToWidgetPosition` _returnvalue _returnvalue_2))) (`KismetMathLibrary.Normal` (- _returnvalue_3 _returnvalue_2))))

(fn `GetClickedPointInPlane`
  (params (mousepoint :type "Vector2D Structure"))
  (returns (IntersectionPoint :type "Vector Structure") (IsIntersect :type Boolean))
  (bind _defaultsceneroot (`self.DefaultSceneRoot`))
  (bind (_worldposition _worlddirection) (`GameplayStatics.DeprojectScreenToWorld` (`GameplayStatics.GetPlayerController` 0) mousepoint))
  (bind (_t _intersection _returnvalue) (`KismetMathLibrary.LinePlaneIntersection` _worldposition (* _worlddirection 100000.0) (`KismetMathLibrary.MakePlaneFromPointAndNormal` (`SceneComponent.K2_GetComponentLocation` _defaultsceneroot) (`.Y` (`KismetMathLibrary.BreakRotIntoAxes` (`SceneComponent.K2_GetComponentRotation` _defaultsceneroot))))))
  (`|ExecutionSequence`
    (:`then_1`
      (return _intersection _returnvalue))))

(fn `GetStartEndVectorsInMarkerCoordinate`
  (returns (Start :type "Vector Structure") (End :type "Vector Structure"))
  (locals (CursurLocation :type "Vector Structure" :default (0.0 0.0 0.0)))
  (bind _defaultsceneroot (`self.DefaultSceneRoot`))
  (bind _returnvalue (`SceneComponent.K2_GetComponentLocation` _defaultsceneroot))
  (bind _hitresult (`PlayerController.GetHitResultUnderCursorByChannel` (`GameplayStatics.GetPlayerController` 0) "TraceTypeQuery3" true))
  (bind _returnvalue_2 (`SceneComponent.K2_GetComponentRotation` _defaultsceneroot))
  (bind _output_get (set `local.CursurLocation` (`self.LastCursurLocation`)))
  (set `self.LastCursurLocation` (`.Location` (`GameplayStatics.BreakHitResult` _hitresult)))
  (return (`KismetMathLibrary.GreaterGreater_VectorRotator` (- _output_get _returnvalue) _returnvalue_2) (`KismetMathLibrary.GreaterGreater_VectorRotator` (- (`.Location` (`GameplayStatics.BreakHitResult` _hitresult)) _returnvalue) _returnvalue_2)))

(fn `GetStartEndVectorsInMarkerCoordinate2`
  (returns (Start :type "Vector Structure") (End :type "Vector Structure"))
  (locals (CursurLocation :type "Vector Structure" :default (0.0 0.0 0.0)))
  (bind _returnvalue (`SceneComponent.K2_GetComponentLocation` (`self.DefaultSceneRoot`)))
  (bind _hitresult (`PlayerController.GetHitResultUnderCursorByChannel` (`GameplayStatics.GetPlayerController` 0) "TraceTypeQuery3" true))
  (bind _returnvalue_2 (`SceneComponent.K2_GetComponentRotation` (`self.SelectedComponent`)))
  (bind _output_get (set `local.CursurLocation` (`self.LastCursurLocation`)))
  (set `self.LastCursurLocation` (`.Location` (`GameplayStatics.BreakHitResult` _hitresult)))
  (return (`KismetMathLibrary.LessLess_VectorRotator` (- _output_get _returnvalue) _returnvalue_2) (`KismetMathLibrary.LessLess_VectorRotator` (- (`.Location` (`GameplayStatics.BreakHitResult` _hitresult)) _returnvalue) _returnvalue_2)))

(fn `PreRotation`
  (params (InVec :type "Vector Structure"))
  (if (not (`self.IsRotationStart`))
    (set `self.IsRotationStart` true)
    (`self.SpawnRotationPlane` (`KismetMathLibrary.Conv_VectorToRotator` InVec))
    (set `self.LastCursurLocation` (`/RapyutaSimulationPlugins/Tools/BP_WidgetPlayer.ClickedMarkerLocation` (cast `/RapyutaSimulationPlugins/Tools/BP_WidgetPlayer` (`GameplayStatics.GetPlayerController` 0) :!pure true))))
  (return))

(fn `PreRotation2`
  (if (not (`self.IsRotationStart`))
    ;[1 1 1] Initialization
    (set `self.IsRotationStart` true)
    (`self.SpawnRotationPlane` (`KismetMathLibrary.Conv_VectorToRotator` (`SceneComponent.GetUpVector` (`self.SelectedComponent`))))
    (set `self.LastCursurLocation` (`/RapyutaSimulationPlugins/Tools/BP_WidgetPlayer.ClickedMarkerLocation` (cast `/RapyutaSimulationPlugins/Tools/BP_WidgetPlayer` (`GameplayStatics.GetPlayerController` 0) :!pure true))))
  (return))

(fn `Released`
  (bind _selectedcomponent (`self.SelectedComponent`))
  (bind _plaeyrpawn (`self.PlaeyrPawn`))
  (bind _rotationplane (`self.RotationPlane`))
  (`KismetSystemLibrary.PrintString` "IM: releaseed")
  (`|ExecutionSequence`
    (:`then_0`
      (set `self.XSelected` false)
      (set `self.YSelected` false)
      (set `self.ZSelected` false)
      (set `self.IsRotationStart` false))
    (:`then_1`
      (`/Engine/EditorBlueprintResources/StandardMacros.IsValid` _plaeyrpawn
        (:`Is Valid`
          (`self.EnableInput` _plaeyrpawn (`GameplayStatics.GetPlayerController` 0)))))
    (:`then_2`
      (if (`KismetSystemLibrary.IsValid` _rotationplane)
        (`self.K2_DestroyActor` _rotationplane)))
    (:`then_3`
      (if (`KismetSystemLibrary.IsValid` _selectedcomponent)
        (`self.SetMaterials` _selectedcomponent (`|MakeMap` "x" "/RapyutaSimulationPlugins/Tools/MI_MarkerRed.MI_MarkerRed" "y" "/RapyutaSimulationPlugins/Tools/MI_MarkerGreen.MI_MarkerGreen" "z" "/RapyutaSimulationPlugins/Tools/MI_MarkerBlue.MI_MarkerBlue" :!type "Name" :!valuetype "MaterialInterface Object Reference"))))))

(fn `RotateByQuat`
  (params (Q :type "Quat Structure (by ref)"))
  (bind (_returnvalue_x _returnvalue_y _returnvalue_z) (`KismetMathLibrary.BreakVector` (`KismetMathLibrary.Quat_Euler` Q)))
  (bind _targetactor (`self.TargetActor`))
  (bind _returnvalue (`KismetMathLibrary.MakeRotator` _returnvalue_x _returnvalue_y _returnvalue_z))
  (`|ExecutionSequence`
    (:`then_0`
      (`SceneComponent.K2_SetWorldRotation` (`self.DefaultSceneRoot`) _returnvalue false false))
    (:`then_1`
      (`/Engine/EditorBlueprintResources/StandardMacros.IsValid` _targetactor
        (:`Is Valid`
          (`SceneComponent.K2_SetWorldRotation` (`Actor.RootComponent` _targetactor) _returnvalue false false)
          (return))))))

(fn `RotateRotatorByAxis`
  (params (Axis :type "Vector Structure") (Angle :type "Float (double-precision)") (InRot :type "Rotator Structure"))
  (returns (ReturnValue :type "Quat Structure"))
  (locals (NewLocalVar_0 :type "Quat Structure"))
  (bind _returnvalue (* Angle 0.5))
  (bind _returnvalue_2 (`KismetMathLibrary.DegSin` _returnvalue))
  (bind _returnvalue_3 (`KismetMathLibrary.Quat_MakeFromEuler` (`KismetMathLibrary.MakeVector` (.roll InRot) (.pitch InRot) (.yaw InRot))))
  (`|ExecutionSequence`
    (:`then_0`
      (bind _output_get (set `local.NewLocalVar_0` _returnvalue_3)))
    (:`then_1`
      (if (not (`KismetMathLibrary.NearlyEqual_FloatFloat` Angle))
        (`KismetSystemLibrary.PrintString` (`KismetStringLibrary.Concat_StrStr` "angle" (`KismetStringLibrary.Conv_DoubleToString` Angle)))
        (`KismetSystemLibrary.PrintString` (`KismetStringLibrary.Concat_StrStr` (`KismetStringLibrary.Concat_StrStr` (`KismetStringLibrary.Concat_StrStr` (`KismetStringLibrary.Concat_StrStr` "x:" (`KismetStringLibrary.Conv_DoubleToString` (`KismetMathLibrary.BreakQuat` _output_get)) ", ") "y: " (`KismetStringLibrary.Conv_DoubleToString` (`.Y` (`KismetMathLibrary.BreakQuat` _output_get))) ", ") "z:" (`KismetStringLibrary.Conv_DoubleToString` (`.Z` (`KismetMathLibrary.BreakQuat` _output_get))) ", ") "w:" (`KismetStringLibrary.Conv_DoubleToString` (`.W` (`KismetMathLibrary.BreakQuat` _output_get)))))))
    (:`then_2`
      (return (* (`KismetMathLibrary.MakeQuat` (* Axis_X _returnvalue_2) (* Axis_Y _returnvalue_2) (* _returnvalue_2 Axis_Z) (`KismetMathLibrary.DegCos` _returnvalue)) _returnvalue_3)))))

(fn `SetMaterials`
  (params (TargetComponent :type "StaticMeshComponent Object Reference") (MaterialList :type "Map of Name to MaterialInterface Object Reference (by ref)"))
  (locals (material :type "MaterialInterface Object Reference" :default "Material'/RapyutaSimulationPlugins/Tools/MI_MarkerRedClicked.MI_MarkerRedClicked'") (NameArray :type "Array of Name"))
  (bind _keys (`BlueprintMapLibrary.Map_Keys` MaterialList))
  (for _array_element _keys
    (if (`ActorComponent.ComponentHasTag` TargetComponent _array_element)
      (for _array_element_2 (`ActorComponent.ComponentTags` TargetComponent)
        (if (`KismetArrayLibrary.Array_Contains` (`local.NameArray`) _array_element_2)
          (for _array_element_3 (`SceneComponent.GetChildrenComponents` (`self.DefaultSceneRoot`) true)
            (if (`ActorComponent.ComponentHasTag` _array_element_3 _array_element_2)
              (if (`ActorComponent.ComponentHasTag` _array_element_3 _array_element)
                (bind _asstatic_mesh_component (cast `StaticMeshComponent` _array_element_3))
                (`PrimitiveComponent.SetMaterial` _asstatic_mesh_component 0 (`BlueprintMapLibrary.Map_Find` MaterialList _array_element))))))))))

(fn `SpawnRotationPlane`
  (params (InRot :type "Rotator Structure"))
  (bind _returnvalue (`|SpawnActorFromClass` "/Script/Engine.StaticMeshActor" (`KismetMathLibrary.MakeTransform` (`SceneComponent.K2_GetComponentLocation` (`self.DefaultSceneRoot`)) InRot (0.001 1000.0 1000.0)) "AlwaysSpawn" "OverrideRootScale" null null))
  (bind _output_get (set `self.RotationPlane` _returnvalue))
  (`|ExecutionSequence`
    (:`then_0`
      (set `Actor.Tags` (`self.Tags_0`) _output_get))
    (:`then_1`
      (`self.SetActorHiddenInGame` _output_get true))
    (:`then_2`
      (bind _staticmeshcomponent (`StaticMeshActor.StaticMeshComponent` _returnvalue))
      (`SceneComponent.SetMobility` _staticmeshcomponent "Movable"))
    (:`then_3`
      (`StaticMeshComponent.SetStaticMesh` _staticmeshcomponent "/RapyutaSimulationPlugins/DynamicContents/StaticMeshes/BasicShapes/Cube.Cube"))
    (:`then_4`
      (`PrimitiveComponent.SetCollisionResponseToChannel` _staticmeshcomponent "ECC_GameTraceChannel1" "ECR_Block"))))

(fn `UserConstructionScript`)