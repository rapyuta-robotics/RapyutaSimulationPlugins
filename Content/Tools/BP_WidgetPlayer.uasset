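; Player controller for a runtime editing tool that creates the WB_RuntimeInteraction UI, toggled with Shift+Space.
; Left clicks trace the marker channel first to drive BP_UIInteractionMoveMarker, then fall back to Visibility to select an actor.
; Actor selection and Delete are broadcast through dispatcher calls.
; F moves the pawn by timeline toward the marker's target, backing off along the camera forward vector by its scaled bounds.
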(event `Key|F`
  (params (Key :type "Key Structure"))
  (:`Pressed`
    (bind _returnvalue (`GameplayStatics.GetActorOfClass` "/RapyutaSimulationPlugins/Tools/BP_UIInteractionMoveMarker.BP_UIInteractionMoveMarker_C"))
    (`/Engine/EditorBlueprintResources/StandardMacros.IsValid` _returnvalue
      (:`Is Valid`
        (`self.FocusToTargetActor` (`/RapyutaSimulationPlugins/Tools/BP_UIInteractionMoveMarker.TargetActor` _returnvalue))))))

(event `self.ReceivePossess`
  (params (PossessedPawn :type "Pawn Object Reference")))

(event `FocusToTargetActor`
  (params (TargetActor :type "Actor Object Reference"))
  (bind _playerlocationbeforfocus (`self.PlayerLocationBeforFocus`))
  (`/Engine/EditorBlueprintResources/StandardMacros.IsValid` TargetActor
    (:`Is Valid`
      (set `self.PlayerLocationBeforFocus` (`self.K2_GetActorLocation` (`self.K2_GetPawn`)))
      (bind (_direction _newtrack_0) (`Timeline|Timeline_0` :!via `PlayFromStart`)
        (:`Update`
          (`self.K2_SetActorLocation` (`self.K2_GetPawn`) (+ (* (- (+ (`self.K2_GetActorLocation` TargetActor) (* (* (`KismetMathLibrary.Normal` (`self.GetActorForwardVector` (`self.PlayerCameraManager`)) 0.1) -1.0) (* (`self.FocusScale`) (`KismetMathLibrary.GetMaxElement` (`.BoxExtent` (`self.GetActorBounds` TargetActor false true)))))) _playerlocationbeforfocus) _newtrack_0) _playerlocationbeforfocus) false false))))))

(event `self.ReceiveBeginPlay`
  (bind _returnvalue (`|CreateWidget` "/RapyutaSimulationPlugins/Widget/WB_RuntimeInteraction.WB_RuntimeInteraction_C"))
  (bind _output_get (set `self.UI` _returnvalue))
  (`UserWidget.AddToViewport` _output_get 0 :!label _label))

(event `Key|Shift+SpaceBar` :paused true
  (params (Key :type "Key Structure"))
  (:`Released`
    (`/Engine/EditorBlueprintResources/StandardMacros.FlipFlop`
      (:`A`
        (`Widget.RemoveFromParent` (`self.UI`)))
      (:`B`
        (goto _label)))))

(event `Key|Delete`
  (params (Key :type "Key Structure"))
  (:`Released`
    (`self.PlayerControllerDeleteReleased`)))

(event `Key|LeftMouseButton`
  (params (Key :type "Key Structure"))
  (bind (_hitresult _returnvalue) (`self.GetHitResultUnderCursorByChannel` "TraceTypeQuery1"))
  (bind (_hitresult_2 _returnvalue_2) (`self.GetHitResultUnderCursorByChannel` "TraceTypeQuery3"))
  (:`Pressed`
    (if (`self.IsClickEnabled`)
      (if _returnvalue_2
        (`|ExecutionSequence`
          (:`then_0`
            (set `self.SelectedInteractiveMarkerComponent` (`.HitComponent` (`GameplayStatics.BreakHitResult` _hitresult_2)))
            (set `self.ClickedMarkerLocation` (`.Location` (`GameplayStatics.BreakHitResult` _hitresult_2)))
            (bind _returnvalue_3 (`GameplayStatics.GetActorOfClass` "/RapyutaSimulationPlugins/Tools/BP_UIInteractionMoveMarker.BP_UIInteractionMoveMarker_C"))
            (`/Engine/EditorBlueprintResources/StandardMacros.IsValid` _returnvalue_3
              (:`Is Valid`
                (`/RapyutaSimulationPlugins/Tools/BP_UIInteractionMoveMarker.IMLeftMouseClicked` _returnvalue_3))))
          (:`then_1`
            ;[1 1 1] debug
            (`KismetSystemLibrary.PrintString` (`KismetStringLibrary.Concat_StrStr` "Interactive marker hit" (`KismetSystemLibrary.GetObjectName` (`.HitComponent` (`GameplayStatics.BreakHitResult` _hitresult_2)))))))
        (elif _returnvalue
          (`|ExecutionSequence`
            (:`then_0`
              (set `self.SelectedActor` (`.HitActor` (`GameplayStatics.BreakHitResult` _hitresult)))
              (set `self.ClickedLocation` (`.ImpactPoint` (`GameplayStatics.BreakHitResult` _hitresult)))
              (`self.PlayerControllerLeftMousePressed`))
            (:`then_1`
              ;[1 1 1] debug
              (`KismetSystemLibrary.PrintString` (`KismetStringLibrary.Concat_StrStr` "non interactive marker hit " (`KismetSystemLibrary.GetObjectName` (`.HitActor` (`GameplayStatics.BreakHitResult` _hitresult)))))))))))
  (:`Released`
    (bind _returnvalue_4 (`GameplayStatics.GetActorOfClass` "/RapyutaSimulationPlugins/Tools/BP_UIInteractionMoveMarker.BP_UIInteractionMoveMarker_C"))
    (`/Engine/EditorBlueprintResources/StandardMacros.IsValid` _returnvalue_4
      (:`Is Valid`
        (`/RapyutaSimulationPlugins/Tools/BP_UIInteractionMoveMarker.IMLeftMousesReleased` _returnvalue_4)))))

(fn `UserConstructionScript`)