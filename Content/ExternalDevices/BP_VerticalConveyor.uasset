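; Vertical conveyor external device that uses a child two-sided elevator to link entrance conveyors on multiple floors.
; Initialization doorlessly configures the elevator and spawns conveyors from the Entrances flags, with index parity choosing the side and index/2 the floor.
; SetTargetEntrance validates an in/out pair, sets elevator floors and sides, then runs only those two conveyors.
; A ROS 2 topic updates the pair at runtime, with sub-devices getting appended namespaces.
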(event `CustomEvent_8`
  (params (InMessage :type "ROS2GenericMsg Object Reference"))
  (bind (_output_layout _output_data) (break `ROSInt32MA` (`ROS2Int32MAMsg.GetMsg` (cast `ROS2Int32MAMsg` InMessage :!pure true))))
  (bind (_result _msg) (`self.SetTargetEntrance` _output_data))
  (`/RapyutaSimulationPlugins/Tools/RRGeneralUtility.Named Log` _msg self))

(event `self.ReceiveBeginPlay`
  (bind _subscriber (`ROS2SubscriberComponent.Subscriber` (`self.SetTargetEntranceSubscriber`)))
  (`parent.ReceiveBeginPlay`)
  (`|ExecutionSequence`
    (:`then_0`
      (bind _res (`self.AddROSNamespace` (`ROS2Topic.TopicName` _subscriber) "set_auto_target_entrances"))
      (set `ROS2Topic.TopicName` _res _subscriber)
      (`ROS2Subscriber.SetDelegates` _subscriber (delegate `CustomEvent_8`))
      (`ROS2NodeComponent.AddSubscription` (`self.ROS2Node`) _subscriber))))

(event `self.BPPreInitializeComponents`
  (bind _elevator (`self.elevator`))
  (set `RRBaseRobot.ROS2Interface` (`self.ROS2Interface`) _elevator)
  (set `/RapyutaSimulationPlugins/ExternalDevices/BP_Elevator2S.AdditionalROSNamespace` (`/RapyutaSimulationPlugins/Tools/RRGeneralUtility.ROSNameAppend` (`self.AdditionalROSNamespace`) "elevator") _elevator)
  (for (_array_element _array_index) (`self.EntranceConveyors`)
    (`/Engine/EditorBlueprintResources/StandardMacros.IsValid` _array_element
      (:`Is Valid`
        (set `RRBaseRobot.ROS2Interface` (`self.ROS2Interface`) _array_element)
        (set `/RapyutaSimulationPlugins/ExternalDevices/BP_Conveyor.AdditionalROSNamespace` (`/RapyutaSimulationPlugins/Tools/RRGeneralUtility.ROSNameAppend` (`self.AdditionalROSNamespace`) (`KismetStringLibrary.Concat_StrStr` "conveyor" (`KismetStringLibrary.Conv_IntToString` _array_index))) _array_element)))))

(fn `Init Entrances`
  (bind _temp_front_back (`self.temp_front_back`))
  (bind (_entranceoffset_x _entranceoffset_y _entranceoffset_z) (`KismetMathLibrary.BreakVector` (`self.EntranceOffset`)))
  (bind _returnvalue_x (`KismetMathLibrary.BreakVector` (`SceneComponent.K2_GetComponentScale` (`self.ChildActor`))))
  (`KismetArrayLibrary.Array_Clear` (`self.EntranceConveyors`))
  (for (_array_element _array_index) (`self.Entrances`)
    (`KismetSystemLibrary.PrintString` (`KismetStringLibrary.Concat_StrStr` "entrance" (`KismetStringLibrary.Conv_IntToString` _array_index)) true true (struct :`G` 0.66 :`B` 1.0 :`A` 1.0) 2.2)
    (if _array_element
      (if (== (mod _array_index 2) 0)
        (set `self.temp_front_back` 1)
        (else
          (set `self.temp_front_back` -1)))
      (bind _returnvalue (`|AddComponentByClass` "/Script/Engine.ChildActorComponent" false (`KismetMathLibrary.MakeTransform` (`KismetMathLibrary.MakeVector` (* (+ _entranceoffset_x (* _returnvalue_x 100.0)) _temp_front_back) 0.0 (+ (* (/ _array_index 2) (`self.FloorHeight`)) _entranceoffset_z)) (`KismetMathLibrary.MakeRotator` 0.0 0.0 (`KismetMathLibrary.Conv_IntToDouble` (+ (* _temp_front_back 90) -90))) (`self.EntranceScale`))))
      (`ChildActorComponent.SetChildActorClass` _returnvalue (`self.EntranceActorClass`))
      (bind _childactor (`ChildActorComponent.ChildActor` _returnvalue))
      (`KismetArrayLibrary.Array_Add` (`self.EntranceConveyors`) (cast `/RapyutaSimulationPlugins/ExternalDevices/BP_Conveyor` _childactor :!pure true))
      (`KismetSystemLibrary.PrintString` (`KismetStringLibrary.Concat_StrStr` "VC Construction " (`KismetSystemLibrary.GetObjectName` _childactor)))
      (for _array_element_2 (`self.EntranceConveyors`)
        (`/RapyutaSimulationPlugins/ExternalDevices/BP_Conveyor.SetVel` _array_element_2 0.0)
        (set `/RapyutaSimulationPlugins/ExternalDevices/BP_Conveyor.DisableGravity` (`self.DisableGravityAtEntrance`) _array_element_2))
      (else
        (`|AddComponentByClass` "/Script/Engine.ChildActorComponent" false (`KismetMathLibrary.MakeTransform` (0.0 0.0 0.0) (`KismetMathLibrary.MakeRotator` 0.0)))
        (`KismetArrayLibrary.Array_Add` (`self.EntranceConveyors`))))))

(fn `InitElev`
  (bind _elevator (`self.elevator`))
  (set `/RapyutaSimulationPlugins/ExternalDevices/BP_Elevator2S.FloorHeight` (`self.FloorHeight`) _elevator)
  (set `/RapyutaSimulationPlugins/ExternalDevices/BP_Elevator2S.Mode` 2 _elevator)
  (set `/RapyutaSimulationPlugins/ExternalDevices/BP_Elevator2S.HasDoor` false _elevator)
  (`/RapyutaSimulationPlugins/ExternalDevices/BP_Elevator2S.DestroyDoor` _elevator)
  (`KismetArrayLibrary.Array_Resize` (`/RapyutaSimulationPlugins/ExternalDevices/BP_Elevator2S.OpenFrontDoorByFloor` _elevator) (/ (`KismetArrayLibrary.Array_Length` (`self.Entrances`)) 2)))

(fn `Initialize`
  (`parent.Initialize`)
  (`self.InitElev`)
  (`self.Init Entrances`)
  (bind (_result _msg) (`self.SetTargetEntrance` (`self.TargetEntrances`)))
  (if _result
    (`KismetSystemLibrary.PrintString` _msg)
    (else
      (`KismetSystemLibrary.PrintString` _msg true true (struct :`R` 1.0 :`A` 1.0) 20.0))))

(fn `InitializeChildActor`
  (`parent.InitializeChildActor`)
  (set `self.elevator` (cast `/RapyutaSimulationPlugins/ExternalDevices/BP_Elevator2S` (`ChildActorComponent.ChildActor` (`self.ChildActor`)) :!pure true))
  (`/RapyutaSimulationPlugins/ExternalDevices/BP_Conveyor.Set Sensor Length` (`/RapyutaSimulationPlugins/ExternalDevices/BP_Elevator2S.Conveyor` (`self.elevator`)) 100.0))

(fn `ResetAllConvSpeed`
  (for _array_element (`self.EntranceConveyors`)
    (`/Engine/EditorBlueprintResources/StandardMacros.IsValid` _array_element
      (:`Is Valid`
        (`/RapyutaSimulationPlugins/ExternalDevices/BP_Conveyor.SetVel` _array_element 0.0)))))

(fn `SetTargetEntrance`
  (params (TargetEntrance :type "Array of Integer"))
  (returns (result :type Boolean) (Msg :type String))
  (locals (res :type Boolean :default false) (ElevTargetFloor :type "Array of Integer") (OutMsg :type String))
  (bind _output (`|GetArrayItem` TargetEntrance))
  (bind _output_2 (`|GetArrayItem` TargetEntrance 1))
  (bind _entranceconveyors (`self.EntranceConveyors`))
  (bind _entrancevel (`self.EntranceVel`))
  (bind _elevtargetfloor (`local.ElevTargetFloor`))
  (bind _targetentrances (`self.TargetEntrances`))
  (bind _entranceconveyors_2 (`self.EntranceConveyors`))
  (bind _openfrontdoorbyfloor (`/RapyutaSimulationPlugins/ExternalDevices/BP_Elevator2S.OpenFrontDoorByFloor` (`self.elevator`)))
  (bind _output_3 (`|GetArrayItem` _entranceconveyors (`|GetArrayItem` _targetentrances 1)))
  (bind _output_4 (`|GetArrayItem` _entranceconveyors (`|GetArrayItem` _targetentrances)))
  (if (or (< (`|GetArrayItem` TargetEntrance) 0) (< (`|GetArrayItem` TargetEntrance 1) 0))
    (`self.ResetAllConvSpeed`)
    (set `self.TargetEntrances` TargetEntrance)
    (else
      (if (!= (`KismetArrayLibrary.Array_Length` (`self.EntranceConveyors`)) (`KismetArrayLibrary.Array_Length` (`self.Entrances`)))
        (set `local.OutMsg` "Entrance and conveyor num is mismuch.")
        (elif (!= (`KismetArrayLibrary.Array_Length` TargetEntrance) 2)
          (set `local.OutMsg` "Target Entrance Length must be two")
          (elif (== _output _output_2)
            (set `local.OutMsg` "Entrance and Exsit is same")
            (else
              (`/Engine/EditorBlueprintResources/StandardMacros.IsValid` (`|GetArrayItem` _entranceconveyors_2 _output)
                (:`Is Valid`
                  (`/Engine/EditorBlueprintResources/StandardMacros.IsValid` (`|GetArrayItem` _entranceconveyors_2 _output_2)
                    (:`Is Valid`
                      (bind _output_get (set `self.TargetEntrances` TargetEntrance))
                      ;[1 1 1] Set Elevator's Auto target floors and Open Front door by floor
                      (`KismetArrayLibrary.Array_Clear` _elevtargetfloor)
                      (for _array_element _output_get
                        (bind _returnvalue (/ _array_element 2))
                        (`KismetArrayLibrary.Array_Add` _elevtargetfloor _returnvalue)
                        (if (== (mod _array_element 2) 0)
                          (`KismetArrayLibrary.Array_Set` _openfrontdoorbyfloor _returnvalue true)
                          (else
                            (`KismetArrayLibrary.Array_Set` _openfrontdoorbyfloor _returnvalue))))
                      (bind (_msg _result) (`/RapyutaSimulationPlugins/ExternalDevices/BP_Elevator2S.SetAutoTargetFloor` (`self.elevator`) (`local.ElevTargetFloor`)))
                      (set `local.OutMsg` _msg)
                      (if _result
                        ;[1 1 1] Set vel=0 for all entrances
                        (`self.ResetAllConvSpeed`)
                        ;[1 1 1] Set Entrance conveyor velocity
                        (set `/RapyutaSimulationPlugins/ExternalDevices/BP_Conveyor.Mode` 0 _output_4)
                        (`/RapyutaSimulationPlugins/ExternalDevices/BP_Conveyor.SetVel` _output_4 (* _entrancevel -1.0))
                        (set `/RapyutaSimulationPlugins/ExternalDevices/BP_Conveyor.Mode` 1 _output_3)
                        (`/RapyutaSimulationPlugins/ExternalDevices/BP_Conveyor.SetVel` _output_3 _entrancevel)
                        (bind _output_get_2 (set `local.res` true))
                        (return _output_get_2 (`local.OutMsg`))
                        (else
                          (bind _output_get_3 (set `local.res` false))
                          (return _output_get_3 (`local.OutMsg`)))))
                    (:`Is Not Valid`
                      _)))
                (:`Is Not Valid`
                  _))
              (set `local.OutMsg` "Given TargetEntrance is not exists")))))
      (bind _output_get_4 (set `local.res` false))
      (return _output_get_4 (`local.OutMsg`)))))

(fn `UserConstructionScript`
  (`parent.UserConstructionScript`))