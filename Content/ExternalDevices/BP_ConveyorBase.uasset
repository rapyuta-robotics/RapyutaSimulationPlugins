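; Base conveyor device, controlled over ROS 2, that moves payload actors along each collision component's forward vector.
; Each tick it offsets actors reported by per-collision addon components, using kinematic moves rather than belt physics.
; Two sensors detect payloads; mode 1 halts transport while the exit-side sensor, picked by velocity sign, is occupied.
; ROS topics set velocity and mode and publish sensor states; JSON parameters configure sensor transforms and speed.
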(event `self.ReceiveTick`
  (params (DeltaSeconds :type "Float (single-precision)"))
  (`self.UpdateStatus`)
  (if (`self.On`)
    (`|ExecutionSequence`
      (:`then_0`
        ;[1 1 1] Mode==1: Stop moving object if something hit the sensor at exit
        (`self.UpdateSensorStatus`)
        (if (> (`self.AutoVel`) 0.0)
          (set `self.TargetSensor` 0)
          (else
            (set `self.TargetSensor` 1)))
        (switch `int` (`self.Mode`)
          (:`Default`
            (set `self.Speed` 0.0 :!label _label))
          (:`0`
            (set `self.Speed` (`self.AutoVel`) :!label _label_2))
          (:`1`
            (if (`self.ObjectAtExit`)
              (goto _label)
              (else
                (goto _label_2))))))
      (:`then_1`
        (`self.MovePayload` DeltaSeconds)))))

(event `CustomEvent`
  (params (InTopicMessage :type "ROS2GenericMsg Object Reference"))
  (`ROS2Int32MAMsg.SetMsg` (cast `ROS2Int32MAMsg` InTopicMessage :!pure true) (make `ROSInt32MA` (make `ROSMALayout` _) (`self.IsSensorDetect`))))

(event `CustomEvent_0`
  (params (InMessage :type "ROS2GenericMsg Object Reference"))
  (bind _output_data (break `ROSFloat32` (`ROS2Float32Msg.GetMsg` (cast `ROS2Float32Msg` InMessage :!pure true))))
  (bind _returnvalue (* _output_data 100.0))
  (`self.SetVel` _returnvalue)
  (`/RapyutaSimulationPlugins/Tools/RRGeneralUtility.Named Log` (`KismetStringLibrary.Concat_StrStr` "speed was changed to " (`KismetStringLibrary.Conv_DoubleToString` _returnvalue)) self))

(event `CustomEvent_1`
  (params (InMessage :type "ROS2GenericMsg Object Reference"))
  (bind _output_data (break `ROSInt32` (`ROS2Int32Msg.GetMsg` (cast `ROS2Int32Msg` InMessage :!pure true))))
  (if (> _output_data 1)
    (`/RapyutaSimulationPlugins/Tools/RRGeneralUtility.Named Log` "Mode must be 0, 1" self :!label _label_3)
    (elif (< _output_data 0)
      (goto _label_3)
      (elif (not (== _output_data (`self.Mode`)))
        (bind _output_get (set `self.Mode` _output_data))
        (`/RapyutaSimulationPlugins/Tools/RRGeneralUtility.Named Log` (`KismetStringLibrary.Concat_StrStr` "mode was changed to" (`KismetStringLibrary.Conv_IntToString` _output_get)) self)))))

(event `self.ReceiveBeginPlay`
  (bind _publisher (`ROS2PublisherComponent.Publisher` (`self.EntranceStatePublisher`)))
  (bind _subscriber (`ROS2SubscriberComponent.Subscriber` (`self.SetModeSubscriber`)))
  (bind _subscriber_2 (`ROS2SubscriberComponent.Subscriber` (`self.SetVelSubscriber`)))
  (`parent.ReceiveBeginPlay`)
  (`|ExecutionSequence`
    (:`then_0`
      (bind _res (`self.AddROSNamespace` (`ROS2Topic.TopicName` _publisher) "entrance"))
      (set `ROS2Topic.TopicName` _res _publisher)
      (`ROS2Publisher.SetDelegates` _publisher (delegate `CustomEvent`))
      (`ROS2NodeComponent.AddPublisher` (`self.ROS2Node`) _publisher))
    (:`then_1`
      (bind _res_2 (`self.AddROSNamespace` (`ROS2Topic.TopicName` _subscriber_2) "set_vel"))
      (set `ROS2Topic.TopicName` _res_2 _subscriber_2)
      (`ROS2Subscriber.SetDelegates` _subscriber_2 (delegate `CustomEvent_0`))
      (`ROS2NodeComponent.AddSubscription` (`self.ROS2Node`) _subscriber_2))
    (:`then_2`
      (bind _res_3 (`self.AddROSNamespace` (`ROS2Topic.TopicName` _subscriber) "set_mode"))
      (set `ROS2Topic.TopicName` _res_3 _subscriber)
      (`ROS2Subscriber.SetDelegates` _subscriber (delegate `CustomEvent_1`))
      (`ROS2NodeComponent.AddSubscription` (`self.ROS2Node`) _subscriber))))

(event `UpdateStatus`
  (set `self.On` (not (`KismetMathLibrary.NearlyEqual_FloatFloat` (`self.AutoVel`) 0.0 0.0001))))

(fn `GetAllCarryingActors`
  (returns (NewParam :type "Array of Actor Object Reference"))
  (locals (NewLocalVar_0 :type "Array of Actor Object Reference") (NewLocalVar :type "Array of Actor Object Reference") (NewLocalVar_1 :type "Array of Actor Object Reference"))
  (bind _newlocalvar (`local.NewLocalVar`))
  (`KismetArrayLibrary.Array_Clear` _newlocalvar)
  (for _array_element (`self.Collisions`)
    (for _array_element_2 (`self.GetCarryingActors` _array_element)
      (`KismetArrayLibrary.Array_AddUnique` _newlocalvar _array_element_2)))
  (return _newlocalvar))

(fn `GetAllOverlappingActors`
  (returns (NewParam :type "Array of Actor Object Reference"))
  (locals (NewLocalVar_0 :type "Array of Actor Object Reference") (NewLocalVar :type "Array of Actor Object Reference") (NewLocalVar_1 :type "Array of Actor Object Reference"))
  (bind _newlocalvar (`local.NewLocalVar`))
  (bind _newlocalvar_1 (`local.NewLocalVar_1`))
  (`KismetArrayLibrary.Array_Clear` (`local.NewLocalVar`))
  (`KismetArrayLibrary.Array_Clear` (`local.NewLocalVar_1`))
  (for _array_element (`self.Collisions`)
    (`KismetArrayLibrary.Array_Append` _newlocalvar_1 (`self.GetCarryingActors` _array_element))
    (`KismetArrayLibrary.Array_Append` _newlocalvar_1 (`self.GetWaitingActors` _array_element))
    (for _array_element_2 _newlocalvar_1
      (`KismetArrayLibrary.Array_AddUnique` _newlocalvar _array_element_2))
    (return _newlocalvar)))

(fn `GetCarryingActors`
  (params (Collision :type "PrimitiveComponent Object Reference"))
  (returns (CarryingActors :type "Array of Actor Object Reference"))
  (bind _asbp_conveyor_collision_mesh_addon (cast `/RapyutaSimulationPlugins/ExternalDevices/BP_ConveyorCollisionMeshAddon` (`RRGeneralUtils.FindChildComponentByClass` Collision "/RapyutaSimulationPlugins/ExternalDevices/BP_ConveyorCollisionMeshAddon.BP_ConveyorCollisionMeshAddon_C" true))
    (:`then`
      (return (`/RapyutaSimulationPlugins/ExternalDevices/BP_ConveyorCollisionMeshAddon.CarryingActors` _asbp_conveyor_collision_mesh_addon)))
    (:`CastFailed`
      (return (`PrimitiveComponent.GetOverlappingActors` Collision "/Script/Engine.Actor")))))

(fn `GetExceptionActors`
  (returns (ExceptionActors :type "Array of Actor Object Reference"))
  (bind _exceptionalactors (`self.ExceptionalActors`))
  (for _array_element (`self.Collisions`)
    (bind _asbp_conveyor_collision_mesh_addon (cast `/RapyutaSimulationPlugins/ExternalDevices/BP_ConveyorCollisionMeshAddon` (`RRGeneralUtils.FindChildComponentByClass` _array_element "/RapyutaSimulationPlugins/ExternalDevices/BP_ConveyorCollisionMeshAddon.BP_ConveyorCollisionMeshAddon_C" true)))
    (for _array_element_2 (`/RapyutaSimulationPlugins/ExternalDevices/BP_ConveyorCollisionMeshAddon.ExceptionActors` _asbp_conveyor_collision_mesh_addon)
      (`KismetArrayLibrary.Array_AddUnique` _exceptionalactors _array_element_2))
    (return _exceptionalactors)))

(fn `GetOverlappingActorsWithoutCheck`
  (returns (NewParam :type "Array of Actor Object Reference"))
  (locals (NewLocalVar_2 :type "Array of Actor Object Reference"))
  (bind _newlocalvar_2 (`local.NewLocalVar_2`))
  (for _array_element (`self.Collisions`)
    (`KismetArrayLibrary.Array_Append` _newlocalvar_2 (`PrimitiveComponent.GetOverlappingActors` _array_element "/Script/Engine.Actor")))
  (return _newlocalvar_2))

(fn `GetWaitingActors`
  (params (Collision :type "PrimitiveComponent Object Reference"))
  (returns (CarryingActors :type "Array of Actor Object Reference"))
  (bind _asbp_conveyor_collision_mesh_addon (cast `/RapyutaSimulationPlugins/ExternalDevices/BP_ConveyorCollisionMeshAddon` (`RRGeneralUtils.FindChildComponentByClass` Collision "/RapyutaSimulationPlugins/ExternalDevices/BP_ConveyorCollisionMeshAddon.BP_ConveyorCollisionMeshAddon_C" true))
    (:`then`
      (return (`/RapyutaSimulationPlugins/ExternalDevices/BP_ConveyorCollisionMeshAddon.WaitingActors` _asbp_conveyor_collision_mesh_addon)))
    (:`CastFailed`
      (return))))

(fn `MovePayload`
  (params (DeltaTime :type "Float (double-precision)"))
  (for _array_element (`self.Collisions`)
    (for _array_element_2 (`self.GetCarryingActors` _array_element)
      (bind _returnvalue (`SceneComponent.GetForwardVector` _array_element))
      (`self.K2_AddActorWorldOffset` _array_element_2 (* _returnvalue (* DeltaTime (`self.Speed`))) false false)
      (`BlueprintMapLibrary.Map_Add` (`self.PayloadsLastVel`) _array_element_2 _returnvalue))))

(fn `ObjectAtExit`
  (returns (ReturnValue :type Boolean))
  (return (> (`|GetArrayItem` (`self.IsSensorDetect`) (`self.TargetSensor`)) 0.0)))

(fn `OnAddPayload`
  (params (Payload :type "Actor Object Reference") (Collision :type "PrimitiveComponent Object Reference")))

(fn `OnRemovePayload`
  (params (Payload :type "Actor Object Reference") (Collision :type "PrimitiveComponent Object Reference"))
  (bind _newparam (`self.GetOverlappingActorsWithoutCheck`))
  (if (not (`KismetArrayLibrary.Array_Contains` _newparam Payload))
    (`BlueprintMapLibrary.Map_Remove` (`self.PayloadsLastVel`) Payload)))

(fn `ParamParserImpl`
  (params (JsonInput :type "JsonObjectWrapper Structure"))
  (`parent.ParamParserImpl` JsonInput)
  (`|ExecutionSequence`
    (:`then_1`
      (bind (_outvalue _returnvalue) (`|GetJsonField` JsonInput "sensor1_transform"))
      (if _returnvalue
        (bind _returnvalue_2 (`RRConversionUtils.TransformUEToROS` _outvalue))
        (`SceneComponent.K2_SetRelativeTransform` (`self.Sensor1`) _returnvalue_2 false false)))
    (:`then_2`
      (bind (_outvalue_2 _returnvalue_3) (`|GetJsonField` JsonInput "sensor2_transform"))
      (if _returnvalue_3
        (bind _returnvalue_4 (`RRConversionUtils.TransformUEToROS` _outvalue_2))
        (`SceneComponent.K2_SetRelativeTransform` (`self.Sensor2`) _returnvalue_4 false false)))
    (:`then_3`
      (`|ExecutionSequence`
        (:`then_0`
          (bind (_outvalue_3 _returnvalue_5) (`|GetJsonField` JsonInput "vel"))
          (if _returnvalue_5
            (`self.SetVel` (* _outvalue_3 100.0))))))))

(fn `PostInitialize`
  (for _array_element (`self.Collisions`)
    (`self.SetupCollision` _array_element)
    (`parent.PostInitialize`)))

(fn `SetDebug`
  (params (debug :type Boolean))
  (`parent.SetDebug` debug)
  (`|ExecutionSequence`
    (:`then_0`
      (for _array_element (`self.Collisions`)
        (bind _asbp_conveyor_collision_mesh_addon (cast `/RapyutaSimulationPlugins/ExternalDevices/BP_ConveyorCollisionMeshAddon` (`RRGeneralUtils.FindChildComponentByClass` _array_element "/RapyutaSimulationPlugins/ExternalDevices/BP_ConveyorCollisionMeshAddon.BP_ConveyorCollisionMeshAddon_C" true)))
        (set `/RapyutaSimulationPlugins/ExternalDevices/BP_ConveyorCollisionMeshAddon.Debug` debug _asbp_conveyor_collision_mesh_addon)))
    (:`then_1`
      (`self.Visible Mesh` debug))))

(fn `SetDisablePhysics`
  (params (disable :type Boolean))
  (`parent.SetDisablePhysics` disable)
  (for _array_element (`self.Collisions`)
    (bind _asbp_conveyor_collision_mesh_addon (cast `/RapyutaSimulationPlugins/ExternalDevices/BP_ConveyorCollisionMeshAddon` (`RRGeneralUtils.FindChildComponentByClass` _array_element "/RapyutaSimulationPlugins/ExternalDevices/BP_ConveyorCollisionMeshAddon.BP_ConveyorCollisionMeshAddon_C" true)))
    (set `/RapyutaSimulationPlugins/ExternalDevices/BP_ConveyorCollisionMeshAddon.DisablePhysics` disable _asbp_conveyor_collision_mesh_addon)))

(fn `SetExceptionActor`
  (params (Actor :type "Actor Object Reference"))
  (bind _exceptionalactors (`self.ExceptionalActors`))
  (`KismetArrayLibrary.Array_AddUnique` _exceptionalactors Actor)
  (for _array_element (`self.Collisions`)
    (bind _asbp_conveyor_collision_mesh_addon (cast `/RapyutaSimulationPlugins/ExternalDevices/BP_ConveyorCollisionMeshAddon` (`RRGeneralUtils.FindChildComponentByClass` _array_element "/RapyutaSimulationPlugins/ExternalDevices/BP_ConveyorCollisionMeshAddon.BP_ConveyorCollisionMeshAddon_C" true)))
    (set `/RapyutaSimulationPlugins/ExternalDevices/BP_ConveyorCollisionMeshAddon.ExceptionActors` _exceptionalactors _asbp_conveyor_collision_mesh_addon)))

(fn `SetupCollision`
  (params (Parent :type "SceneComponent Object Reference"))
  (bind _returnvalue (`AddComponent|NODE_AddBP_ConveyorCollisionMeshAddon-0`))
  (`SceneComponent.K2_AttachToComponent` _returnvalue Parent "None" "KeepRelative" "KeepRelative" "KeepRelative" true)
  (`|ExecutionSequence`
    (:`then_0`
      (set `/RapyutaSimulationPlugins/ExternalDevices/BP_ConveyorCollisionMeshAddon.Tag` (`self.Tag`) _returnvalue))
    (:`then_1`
      (set `/RapyutaSimulationPlugins/ExternalDevices/BP_ConveyorCollisionMeshAddon.ExceptionTag` (`self.ExceptionTag`) _returnvalue))
    (:`then_2`
      (set `/RapyutaSimulationPlugins/ExternalDevices/BP_ConveyorCollisionMeshAddon.MaxPayload` (`self.MaxPayload`) _returnvalue))))

(fn `SetVel`
  (params (AutoVel :type "Float (double-precision)"))
  (bind _output_get (set `self.AutoVel` AutoVel))
  (set `self.Speed` _output_get))

(fn `UpdateSensorStatus`
  (locals (Sensors :type "Array of StaticMeshComponent Object Reference") (SensorStatus :type "Array of Integer"))
  (bind _sensors (`local.Sensors`))
  (bind _sensorstatus (`local.SensorStatus`))
  (`KismetArrayLibrary.Array_Clear` _sensors)
  (`KismetArrayLibrary.Array_Add` _sensors (`self.Sensor1`))
  (`KismetArrayLibrary.Array_Add` _sensors (`self.Sensor2`))
  (`KismetArrayLibrary.Array_Clear` _sensorstatus)
  (`KismetArrayLibrary.Array_Resize` _sensorstatus 2)
  (for (_array_element _array_index) _sensors
    (for _array_element_2 (`PrimitiveComponent.GetOverlappingActors` _array_element "/Script/Engine.Actor")
      (bind _result (`/RapyutaSimulationPlugins/Tools/RRGeneralUtility.Check Payload` self _array_element_2 (`self.GetExceptionActors`) (`self.Tag`) (`self.ExceptionTag`)))
      (if _result
        (`KismetArrayLibrary.Array_Set` (`local.SensorStatus`) _array_index 1)
        (break))))
  (set `self.IsSensorDetect` (`local.SensorStatus`)))

(fn `UserConstructionScript`
  (`parent.UserConstructionScript`))

(fn `Visible Mesh`
  (params (Visibility :type Boolean))
  (`|ExecutionSequence`
    (:`then_0`
      (`SceneComponent.SetVisibility` (`self.Sensor1`) Visibility true))
    (:`then_1`
      (`SceneComponent.SetVisibility` (`self.Sensor2`) Visibility true))
    (:`then_2`
      (for _array_element (`self.Collisions`)
        (`SceneComponent.SetVisibility` _array_element Visibility true)))))