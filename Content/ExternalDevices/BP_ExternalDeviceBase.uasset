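; Base Blueprint for external devices with ROS 2 integration, providing shared setup, JSON config parsing and topic naming.
; Devices spawned from ROS parse their spawn JSON (or test input in debug) before Initialize; others initialize in the construction script.
; The parser stores "ros" overrides, which AddROSNamespace resolves by key and prefixes with an optional namespace.
; ROSSetup, Initialize, InitializeChildActor and ParamParserImpl are empty hooks for subclasses.
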(event `self.BPInitPropertiesFromJSON`
  ;[1 1 1] Initialize if it is spawn from ROS.
  ; Initialize in InitializeWithoutROSSpawnParameter function If it is not spawn from ROS.
  (`KismetSystemLibrary.PrintString` "BPInitPropertiesFromJson" true true (struct :`G` 0.66 :`B` 1.0 :`A` 1.0) 2000.0)
  (if (`self.ParseParamFromJson`)
    (if (`self.DebugParamParser`)
      (`self.ParamParser` (`self.TestJsonInput`))
      (else
        (`self.ParamParser` (`ROS2Spawnable.ActorJsonConfigs` (`self.ROSSpawnParameters`)))))
    (`self.Initialize`)))

(event `self.ReceiveBeginPlay`
  (set `self.ROS2Node` (`RRRobotROS2Interface.RobotROS2Node` (`self.ROS2Interface`))))

(fn `AddROSNamespace`
  (params (Default :type String) (Key :type String))
  (returns (Res :type String))
  (locals (Result :type String))
  (bind _additionalrosnamespace (`self.AdditionalROSNamespace`))
  (bind (_value _returnvalue) (`BlueprintMapLibrary.Map_Find` (`self.ROSParams`) Key))
  (set `local.result` Default)
  (if _returnvalue
    (set `local.result` _value))
  (if (not (`KismetStringLibrary.IsEmpty` _additionalrosnamespace))
    (set `local.Result` (`KismetStringLibrary.Concat_StrStr` _additionalrosnamespace "/" (`local.Result`))))
  (return (`local.Result`)))

(fn `Initialize`)

(fn `InitializeChildActor`)

(fn `ParamParser`
  (params (JsonString :type String))
  (bind _outjsonobject (`JsonBlueprintFunctionLibrary.FromString` JsonString))
  (`|ExecutionSequence`
    (:`then_0`
      (bind (_outvalue _returnvalue) (`|GetJsonField` _outjsonobject "ros"))
      (if _returnvalue
        (set `self.ROSParams` _outvalue)))
    (:`then_1`
      (`self.ParamParserImpl` _outjsonobject))))

(fn `ParamParserImpl`
  (params (JsonInput :type "JsonObjectWrapper Structure")))

(fn `ROSSetup`)

(fn `UserConstructionScript`
  (`self.InitializeChildActor`)
  ;[1 1 1] Initialize if it is not spawn from ROS.
  ; Initialize in ParamParser function If it is spawn from ROS.
  (`/Engine/EditorBlueprintResources/StandardMacros.IsValid` (`self.ROSSpawnParameters`)
    (:`Is Not Valid`
      (`self.Initialize`))))