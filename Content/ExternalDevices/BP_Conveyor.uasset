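; Conveyor external-device Blueprint with a main collision box and two sensor volumes, configured from JSON parameters.
; Construction registers the collision in the Collisions list, and Initialize applies the current sensor length.
; SetSensorLength sizes both sensors to that length and the collision's cross-section, placing them flush inside its opposite X ends.
; The parser override applies "sensor_length", converted from meters, only without "sensor1_transform"; both transform checks read that same field.
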(fn `Initialize`
  (`parent.Initialize`)
  (`self.Set Sensor Length` (`self.SensorLength`)))

(fn `ParamParserImpl`
  (params (JsonInput :type "JsonObjectWrapper Structure"))
  (locals (NewLocalVar :type "Transform Structure"))
  (`parent.ParamParserImpl` JsonInput)
  (`|ExecutionSequence`
    (:`then_1`
      ;[1 1 1] Calc SensorLength if sensor pose params are not given
      (bind (_outvalue _returnvalue) (`|GetJsonField` JsonInput "sensor_length"))
      (bind (_outvalue_2 _returnvalue_2) (`|GetJsonField` JsonInput "sensor1_transform"))
      (bind (_outvalue_3 _returnvalue_3) (`|GetJsonField` JsonInput "sensor1_transform"))
      (set `local.NewLocalVar` _outvalue_2)
      (set `local.NewLocalVar` _outvalue_3)
      (if (and _returnvalue (not (or _returnvalue_2 _returnvalue_3)))
        (`self.Set Sensor Length` (* _outvalue 100.0))))))

(fn `Set Sensor Length`
  (params (SensorLength :type "Float (double-precision)"))
  (bind _collision (`self.Collision`))
  (bind _sensor2 (`self.Sensor2`))
  (bind _sensor1 (`self.Sensor1`))
  (bind _sensor2_2 (`self.Sensor2`))
  (bind _sensor1_2 (`self.Sensor1`))
  (bind _sensor2_3 (`self.Sensor2`))
  (bind _sensor1_3 (`self.Sensor1`))
  (bind _returnvalue_x (`KismetMathLibrary.BreakVector` (`SceneComponent.K2_GetComponentScale` _sensor1_2)))
  (bind _returnvalue_x_2 (`KismetMathLibrary.BreakVector` (`SceneComponent.K2_GetComponentScale` _sensor2_3)))
  (bind (_returnvalue_x_3 _returnvalue_y _returnvalue_z) (`KismetMathLibrary.BreakVector` (`SceneComponent.K2_GetComponentScale` _sensor1)))
  (bind (_returnvalue_x_4 _returnvalue_y_2 _returnvalue_z_2) (`KismetMathLibrary.BreakVector` (`SceneComponent.K2_GetComponentScale` _sensor2_2)))
  (bind (_returnvalue_x_5 _returnvalue_y_3 _returnvalue_z_3) (`KismetMathLibrary.BreakVector` (`SceneComponent.K2_GetComponentScale` (`self.Collision`))))
  (bind (_relativelocation_x _relativelocation_y _relativelocation_z) (`KismetMathLibrary.BreakVector` (`SceneComponent.RelativeLocation` _collision)))
  (bind _relativescale3d_x (`KismetMathLibrary.BreakVector` (`SceneComponent.RelativeScale3D` _collision)))
  (bind _relativescale3d_x_2 (`KismetMathLibrary.BreakVector` (`SceneComponent.RelativeScale3D` _sensor2)))
  (bind _relativescale3d_x_3 (`KismetMathLibrary.BreakVector` (`SceneComponent.RelativeScale3D` _sensor1_3)))
  (bind _returnvalue (* _relativescale3d_x 50.0))
  (bind _output_get (set `self.SensorLength` SensorLength))
  (bind _returnvalue_2 (/ _output_get 100.0))
  (`SceneComponent.SetWorldScale3D` _sensor1 (`KismetMathLibrary.MakeVector` _returnvalue_2 _returnvalue_y _returnvalue_z))
  (`SceneComponent.SetWorldScale3D` _sensor2_2 (`KismetMathLibrary.MakeVector` _returnvalue_2 _returnvalue_y_2 _returnvalue_z_2))
  ;[1 1 1] Resize sensors based on main collision size changes
  (`SceneComponent.SetWorldScale3D` _sensor1_2 (`KismetMathLibrary.MakeVector` _returnvalue_x _returnvalue_y_3 _returnvalue_z_3))
  (`SceneComponent.SetWorldScale3D` _sensor2_3 (`KismetMathLibrary.MakeVector` _returnvalue_x_2 _returnvalue_y_3 _returnvalue_z_3))
  (`SceneComponent.K2_SetRelativeLocation` _sensor1_3 (`KismetMathLibrary.MakeVector` (- _returnvalue (* _relativescale3d_x_3 50.0)) _relativelocation_y _relativelocation_z) false false)
  (`SceneComponent.K2_SetRelativeLocation` _sensor2 (`KismetMathLibrary.MakeVector` (- (* _relativescale3d_x_2 50.0) _returnvalue) _relativelocation_y _relativelocation_z) false false))

(fn `UserConstructionScript`
  (bind _collisions (`self.Collisions`))
  (`KismetArrayLibrary.Array_Clear` _collisions)
  (`KismetArrayLibrary.Array_AddUnique` _collisions (`self.Collision`))
  (`parent.UserConstructionScript`))